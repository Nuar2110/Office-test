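; Elevator button panel actor with three floor buttons that visually shift when selected.
; BeginPlay gathers the button components into an array, which a custom event loops over to return them all to zero relative location.
; The interaction interface event stores the floor state, picks the matching button and snaps it along local Y.
; Neither elevator movement nor the call to reset happens in this graph.
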(event Custom|CE_ResetButtonLoc
  (for _array_element (Variables|Default|Get%20ArrayButtons)
    (Transformation|SetRelativeLocation _array_element "0, 0, 0" false false)))

(event Collision|EventActorBeginOverlap
  (params (OtherActor :type Actor%20Object%20Reference)))

(event EventTick
  (params (DeltaSeconds :type Float%20%28single-precision%29)))

(event EventBPIInteractionObjects
  (params (InteractState :type String))
  (bind _output_get (Variables|Default|SetInteract%20State InteractState))
  (Utilities|FlowControl|Sequence
    (:then_0
      (switch string _output_get
        (:Floor1
          (Variables|Default|SetTarget (Variables|Default|Get1)))
        (:Floor2
          (Variables|Default|SetTarget (Variables|Default|Get2)))
        (:Floor3
          (Variables|Default|SetTarget (Variables|Default|Get3)))))
    (:then_1
      (Transformation|SetRelativeLocation (Variables|Default|GetTarget) "0.000000,35.000000,0.000000" false false))))

(event EventBeginPlay
  (Variables|Default|Set%20ArrayButtons (Utilities|Array|MakeArray (Variables|Default|Get1) (Variables|Default|Get2) (Variables|Default|Get3))))

(fn ConstructionScript)